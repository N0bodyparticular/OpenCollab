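; BP_PlayerCharacter is a player character Blueprint providing basic movement, mouse look and jumping.
; Forward and Right axes feed the camera's forward and right vectors, without flattening, straight into CharacterMovement as input.
; Look axes add frame-time-scaled yaw and pitch, both using XMouseSensitivity, with InvertMouse choosing the pitch sign.
; The Jump action starts a jump on press and stops it on release.
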(event `InputAxis|Forward`
  (params (AxisValue :type "Float (single-precision)"))
  ;[1 1 1] Basic movment
  (`PawnMovementComponent.AddInputVector` (`self.CharacterMovement`) (* (`SceneComponent.GetForwardVector` (`self.Camera`)) AxisValue) false))

(event `InputAxis|LookRight`
  (params (AxisValue :type "Float (single-precision)"))
  (`self.AddControllerYawInput` (* AxisValue (`self.XMouseSensitivity`) (`GameplayStatics.GetWorldDeltaSeconds`))))

(event `InputAxis|LookUp`
  (params (AxisValue :type "Float (single-precision)"))
  (`self.AddControllerPitchInput` (* AxisValue (`self.XMouseSensitivity`) (`GameplayStatics.GetWorldDeltaSeconds`) (`KismetMathLibrary.SelectFloat` 1.0 -1.0 (`self.InvertMouse`)))))

(event `InputAxis|Right`
  (params (AxisValue :type "Float (single-precision)"))
  ;[1 1 1] Basic movment
  (`PawnMovementComponent.AddInputVector` (`self.CharacterMovement`) (* (`SceneComponent.GetRightVector` (`self.Camera`)) AxisValue) false))

(event `InputAction|Jump`
  (params (Key :type "Key Structure"))
  ;[1 1 1] Basic movment
  (:`Pressed`
    (`self.Jump`))
  (:`Released`
    (`self.StopJumping`)))

(fn `UserConstructionScript`)